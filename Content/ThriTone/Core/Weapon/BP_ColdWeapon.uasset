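; BP_ColdWeapon is a melee weapon that deals fixed damage to actors its Box collision overlaps, ignoring its owner.
; EnableDamage turns on query collision on the Box, and DisableDamage turns it off and clears the hit list.
; Each overlapped actor is added uniquely to OverlapedActors, so it takes damage only once per damage window, with its name printed for debugging.
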(event `self.Box.OnComponentBeginOverlap`
  (params (OverlappedComponent :type "PrimitiveComponent Object Reference") (OtherActor :type "Actor Object Reference") (OtherComp :type "PrimitiveComponent Object Reference") (OtherBodyIndex :type Integer) (bFromSweep :type Boolean) (SweepResult :type "HitResult Structure (by ref)"))
  (if (!= OtherActor (`self.GetOwner`))
    (bind _returnvalue (`KismetArrayLibrary.Array_AddUnique` (`self.OverlapedActors`) OtherActor))
    (if (!= _returnvalue -1)
      (`KismetSystemLibrary.PrintString` (`KismetSystemLibrary.GetDisplayName` OtherActor))
      (`GameplayStatics.ApplyDamage` OtherActor 15.0))))

(fn `DisableDamage`
  (`PrimitiveComponent.SetCollisionEnabled` (`self.Box`) "NoCollision")
  (`KismetArrayLibrary.Array_Clear` (`self.OverlapedActors`)))

(fn `EnableDamage`
  (`PrimitiveComponent.SetCollisionEnabled` (`self.Box`) "QueryOnly"))

(fn `UserConstructionScript`)