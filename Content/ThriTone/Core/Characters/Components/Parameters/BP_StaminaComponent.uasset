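; Stamina parameter component that drains stamina while its owner sprints.
; SprintStart sets a looping timer, guarded against duplicates by a handle check, and SprintEnd clears and invalidates it.
; Sprinting reads the owner's speed through an interface message and, above a small movement threshold, calls DecreaseParameter with consumption scaled by the tick interval.
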(fn `SprintEnd`
  (`KismetSystemLibrary.K2_ClearAndInvalidateTimerHandle` (`self.SprintHandle`))
  (return))

(fn `Sprinting`
  (bind _currentspeed (message `/Game/ThriTone/Core/Interfaces/BPI_Character.GetPlayerSpeed` (`self.GetOwner`)))
  (if (> _currentspeed 30.0)
    (`self.DecreaseParameter` (* (`self.SprintConsumptionValue`) (`self.SprintTick`)))
    (return)))

(fn `SprintStart`
  (if (not (`KismetSystemLibrary.K2_IsValidTimerHandle` (`self.SprintHandle`)))
    (bind _returnvalue (`KismetSystemLibrary.K2_SetTimerDelegate` (`|CreateDelegate` :!event `Sprinting`) (`self.SprintTick`) true))
    (set `self.SprintHandle` _returnvalue)
    (return)
    (else
      (return))))