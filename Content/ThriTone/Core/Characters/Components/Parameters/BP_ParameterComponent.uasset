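; BP_ParameterComponent is a component holding a tagged numeric parameter with minimum and maximum bounds, starting at maximum on BeginPlay.
; Every write goes through SetCurrentParameter, which broadcasts the current value, maximum and tag.
; Increases clamp at maximum and fire a full event; decreases reaching minimum clamp and fire an empty event.
; Decreases staying above minimum set the value to zero rather than the subtracted result.
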(event `self.ReceiveBeginPlay`
  (`self.SetCurrentParameter` (`self.MaxParameterValue`)))

(fn `DecreaseParameter`
  (params (Value :type "Float (double-precision)"))
  (bind _result (`self.HaveParameter` (- (`self.CurrentParameterValue`) Value)))
  (if _result
    (`self.SetCurrentParameter` 0.0)
    (else
      (`self.OnParameterEmpty`))))

(fn `HaveParameter`
  (params (CurrentAmount :type "Float (double-precision)"))
  (returns (Result :type Boolean))
  (return (> CurrentAmount (`self.MinParameterValue`))))

(fn `IncreaseParameter`
  (params (Value :type "Float (double-precision)"))
  (bind _returnvalue (+ (`self.CurrentParameterValue`) Value))
  (if (>= _returnvalue (`self.MaxParameterValue`))
    (`self.OnParameterFull`)
    (else
      (`self.SetCurrentParameter` _returnvalue)))
  (return))

(fn `OnParameterEmpty`
  (`self.SetCurrentParameter` (`self.MinParameterValue`))
  (`self.OnEmptyParameter`)
  (return))

(fn `OnParameterFull`
  (`self.SetCurrentParameter` (`self.MaxParameterValue`))
  (`self.OnFullParameter`)
  (return))

(fn `SetCurrentParameter`
  (params (Value :type "Float (double-precision)"))
  (bind _output_get (set `self.CurrentParameterValue` Value))
  (`self.OnChangedParameter` _output_get (`self.MaxParameterValue`) (`self.ParameterTag`))
  (return))