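; Base player controller that routes Enhanced Input to the pawn it possesses.
; BeginPlay adds the default mapping context, and Possess caches the pawn.
; Look, move, sprint, jump and attack actions are forwarded to that pawn as message calls, with start and release states for sprint and jump.
; HUD widget creation logic is present but unconnected, so it never runs.
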(event `self.ReceiveBeginPlay`
  (bind _returnvalue (pcsubsystem `EnhancedInputLocalPlayerSubsystem` self))
  (`/Engine/EditorBlueprintResources/StandardMacros.IsValid` _returnvalue
    (:`Is Valid`
      (`EnhancedInputSubsystemInterface.AddMappingContext` _returnvalue "/Game/ThriTone/Core/Input/IMC_Default.IMC_Default" 0 (struct)))))

(event `self.ReceivePossess`
  (params (PossessedPawn :type "Pawn Object Reference"))
  (set `self.Possessed Pawn` PossessedPawn))

(event `EnhancedInput|/Game/ThriTone/Core/Input/Actions/IA_Look`
  (params (ActionValue :type "Vector2D Structure") (ElapsedSeconds :type "Float (double-precision)") (TriggeredSeconds :type "Float (double-precision)") (InputAction :type "InputAction Object Reference" :default "/Game/ThriTone/Core/Input/Actions/IA_Look.IA_Look"))
  (:`Triggered`
    (message `/Game/ThriTone/Core/Interfaces/BPI_Character.LookPlayer` (`self.Possessed Pawn`) ActionValue)))

(event `EnhancedInput|/Game/ThriTone/Core/Input/Actions/IA_Sprint`
  (params (ActionValue :type Boolean) (ElapsedSeconds :type "Float (double-precision)") (TriggeredSeconds :type "Float (double-precision)") (InputAction :type "InputAction Object Reference" :default "/Game/ThriTone/Core/Input/Actions/IA_Sprint.IA_Sprint"))
  (:`Started`
    (message `/Game/ThriTone/Core/Interfaces/BPI_Character.Sprint` (`self.Possessed Pawn`) true))
  (:`Completed`
    (message `/Game/ThriTone/Core/Interfaces/BPI_Character.Sprint` (`self.Possessed Pawn`) false)))

(event `EnhancedInput|/Game/ThriTone/Core/Input/Actions/IA_Move`
  (params (ActionValue :type "Vector2D Structure") (ElapsedSeconds :type "Float (double-precision)") (TriggeredSeconds :type "Float (double-precision)") (InputAction :type "InputAction Object Reference" :default "/Game/ThriTone/Core/Input/Actions/IA_Move.IA_Move"))
  (:`Triggered`
    (message `/Game/ThriTone/Core/Interfaces/BPI_Character.MovePlayer` (`self.Possessed Pawn`) ActionValue)))

(event `EnhancedInput|/Game/ThriTone/Core/Input/Actions/IA_Attack`
  (params (ActionValue :type Boolean) (ElapsedSeconds :type "Float (double-precision)") (TriggeredSeconds :type "Float (double-precision)") (InputAction :type "InputAction Object Reference" :default "/Game/ThriTone/Core/Input/Actions/IA_Attack.IA_Attack"))
  (:`Started`
    (message `/Game/ThriTone/Core/Interfaces/BPI_Character.LBM` (`self.Possessed Pawn`))))

(event `EnhancedInput|/Game/ThriTone/Core/Input/Actions/IA_Jump`
  (params (ActionValue :type Boolean) (ElapsedSeconds :type "Float (double-precision)") (TriggeredSeconds :type "Float (double-precision)") (InputAction :type "InputAction Object Reference" :default "/Game/ThriTone/Core/Input/Actions/IA_Jump.IA_Jump"))
  (:`Started`
    (message `/Game/ThriTone/Core/Interfaces/BPI_Character.JumpPlayer` (`self.Possessed Pawn`) true))
  (:`Completed`
    (message `/Game/ThriTone/Core/Interfaces/BPI_Character.JumpPlayer` (`self.Possessed Pawn`) false)))

(fn `UserConstructionScript`
  (`parent.UserConstructionScript`))