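; Base humanoid character Blueprint that provides a starting weapon, damage handling and gameplay tag helpers.
; On BeginPlay it spawns the StartWeaponClass actor, stores it as CurrentWeapon and attaches it to the mesh at the socket the weapon defines.
; AnyDamage lowers the value in BPHealthComponent and prints the damage amount to screen.
; Helper functions add, remove and query (non-exact match) tags in its GTC gameplay tag container.
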(event `self.ReceiveBeginPlay`
  (`self.AddWeapon` (`self.StartWeaponClass`)))

(event `self.ReceiveAnyDamage`
  (params (Damage :type "Float (single-precision)") (DamageType :type "DamageType Object Reference") (InstigatedBy :type "Controller Object Reference") (DamageCauser :type "Actor Object Reference"))
  (`/Game/ThriTone/Core/Characters/Components/Parameters/BP_ParameterComponent.DecreaseParameter` (`self.BP_HealthComponent`) Damage)
  (`KismetSystemLibrary.PrintString` (`KismetStringLibrary.Conv_DoubleToString` Damage) true true (struct :`G` 0.66 :`B` 1.0 :`A` 1.0) 5.0))

(fn `AddWeapon`
  (params (StartWeapon :type "/Game/ThriTone/Core/Weapon/BP_WeaponBase Class Reference"))
  (returns (ReturnValue :type Boolean))
  (bind _returnvalue (`KismetSystemLibrary.IsValidClass` StartWeapon))
  (if _returnvalue
    (bind _returnvalue_2 (`|SpawnActorFromClass` StartWeapon (`KismetMathLibrary.MakeTransform` (0.0 0.0 0.0)) "Undefined" "OverrideRootScale" self null))
    (bind _asbp_weapon_base (cast `/Game/ThriTone/Core/Weapon/BP_WeaponBase` _returnvalue_2))
    (bind _output_get (set `self.CurrentWeapon` _asbp_weapon_base))
    (`self.K2_AttachToComponent` _output_get (`self.Mesh`) (`/Game/ThriTone/Core/Weapon/BP_WeaponBase.WeaponSocket` _output_get) "SnapToTarget" "SnapToTarget" "KeepRelative" true)
    (return _returnvalue)))

(fn `ApplyTagToActor`
  (params (TagToAdd :type "GameplayTag Structure"))
  (returns (Result :type Boolean))
  (`BlueprintGameplayTagLibrary.AddGameplayTag` (`self.GTC`) TagToAdd)
  (return true))

(fn `HasGT`
  (params (TagToCompare :type "GameplayTag Structure"))
  (returns (Result :type Boolean))
  (return (`BlueprintGameplayTagLibrary.HasTag` (`self.GTC`) TagToCompare)))

(fn `RemoveTagFromActor`
  (params (TagToRemove :type "GameplayTag Structure"))
  (returns (Result :type Boolean))
  (bind _returnvalue (`BlueprintGameplayTagLibrary.RemoveGameplayTag` (`self.GTC`) TagToRemove))
  (return _returnvalue))

(fn `UserConstructionScript`)