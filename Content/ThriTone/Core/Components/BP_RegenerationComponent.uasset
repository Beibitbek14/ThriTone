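; BP_RegenerationComponent is a parameter component that automatically refills its value over time after it is decreased.
; A looping tick timer adds the regeneration rate scaled by the tick interval.
; Decreasing the parameter stops regeneration and restarts a delay timer, while reaching full stops both timers.
; AllowRegeneration and AbortRegeneration toggle the flag gating both timers, starting or stopping regeneration immediately.
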(fn `AbortRegeneration`
  (set `self.bCanRegeneration` false)
  (`self.StopRegeneration`))

(fn `AllowRegeneration`
  (set `self.bCanRegeneration` true)
  (`self.StartRegeneration`))

(fn `DecreaseParameter`
  (params (Value :type "Float (double-precision)"))
  (`parent.DecreaseParameter` Value)
  (`self.StopRegeneration`)
  (`self.StartDelayBeforeRegenerate`))

(fn `OnParameterFull`
  (`parent.OnParameterFull`)
  (`self.StopRegeneration`))

(fn `Regeneration`
  (`self.IncreaseParameter` (* (`self.RegenerationValue`) (`self.RegenerationTick`))))

(fn `StartDelayBeforeRegenerate`
  (if (`self.bCanRegeneration`)
    (bind _returnvalue (`KismetSystemLibrary.K2_SetTimerDelegate` (`|CreateDelegate` :!event `StartRegeneration`) (`self.RegenerationDelay`)))
    (set `self.RegenerationDelayHandle` _returnvalue)
    (return)
    (else
      (return))))

(fn `StartRegeneration`
  (if (`self.bCanRegeneration`)
    (bind _returnvalue (`KismetSystemLibrary.K2_SetTimerDelegate` (`|CreateDelegate` :!event `Regeneration`) (`self.RegenerationTick`) true))
    (set `self.RegenerationHandle` _returnvalue)
    (return)
    (else
      (return))))

(fn `StopRegeneration`
  (`KismetSystemLibrary.K2_ClearAndInvalidateTimerHandle` (`self.RegenerationHandle`))
  (`KismetSystemLibrary.K2_ClearAndInvalidateTimerHandle` (`self.RegenerationDelayHandle`))
  (return))